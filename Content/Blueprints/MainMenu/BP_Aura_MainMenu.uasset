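; Main menu scene actor that starts the menu music, shows the WBP_MainMenu widget and animates decorative fire and magic circle components.
; On BeginPlay it creates the widget, switches input to UI-only with the mouse cursor visible, and plays a timeline that moves Fire vertically through scaled world offsets.
; Tick slowly rolls the MagicCircle in local space, scaled by delta time.
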(event `self.ReceiveBeginPlay`
  (bind _returnvalue (`GameplayStatics.GetPlayerController` 0))
  (`GameplayStatics.PlaySound2D` "/Game/Assets/Sounds/Music/Music_MainMenu.Music_MainMenu" 1.0 1.0 0.0 null null)
  (bind _returnvalue_2 (`|CreateWidget` "/Game/Blueprints/UI/MainMenu/WBP_MainMenu.WBP_MainMenu_C"))
  (`UserWidget.AddToViewport` _returnvalue_2 0)
  (`WidgetBlueprintLibrary.SetInputMode_UIOnlyEx` _returnvalue _returnvalue_2)
  (set `PlayerController.bShowMouseCursor` true _returnvalue)
  (bind (_direction _z_axis) (`Timeline|FireUpAndDown`)
    (:`Update`
      (`SceneComponent.K2_AddWorldOffset` (`self.Fire`) (`KismetMathLibrary.MakeVector` 0.0 0.0 (* _z_axis 0.15)) false false))))

(event `self.ReceiveTick`
  (params (DeltaSeconds :type "Float (single-precision)"))
  (`SceneComponent.K2_AddLocalRotation` (`self.MagicCircle`) (`KismetMathLibrary.MakeRotator` (* DeltaSeconds 2.0)) false false))

(fn `UserConstructionScript`)