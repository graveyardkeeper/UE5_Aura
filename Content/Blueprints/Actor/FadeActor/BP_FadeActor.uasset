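; BP_FadeActor is a static mesh actor that can fade out and back in through a material "Fade" parameter.
; Construction caches the original materials and creates dynamic instances from configured fade materials, which FadeOut swaps onto the mesh.
; One timeline drives the parameter, played forward for FadeOut and reversed for Fadein.
; On finish, full Fade restores the original materials, and optional Visibility-channel blocking follows the fade state.
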(event `/Game/Blueprints/Actor/FadeActor/BI_FadeInterface.FadeOut`
  (`self.SetMaterialToDynamicInstance`)
  (bind (_direction _fade) (`Timeline|FadeTimeline` :!via `PlayFromStart` :!label _label)
    (:`Update`
      (for _array_element (`self.DynamicMaterialsInstances`)
        (`MaterialInstanceDynamic.SetScalarParameterValue` _array_element "Fade" _fade)))
    (:`Finished`
      (`self.FadeFinished` _fade))))

(event `/Game/Blueprints/Actor/FadeActor/BI_FadeInterface.FadeIn`
  (goto _label :!via `ReverseFromEnd`))

(event `self.ReceiveBeginPlay`
  (if (`self.ShouldBlockVisibility`)
    (`PrimitiveComponent.SetCollisionResponseToChannel` (`self.StaticMesh`) "ECC_Visibility" "ECR_Block")))

(fn `FadeFinished`
  (params (A :type "Float (double-precision)"))
  (if (>= A 1.0)
    (`self.ResetMaterials`)
    (if (`self.ShouldBlockVisibility`)
      (`PrimitiveComponent.SetCollisionResponseToChannel` (`self.StaticMesh`) "ECC_Visibility" "ECR_Block"))
    (elif (<= A 0.0)
      (if (`self.ShouldBlockVisibility`)
        (`PrimitiveComponent.SetCollisionResponseToChannel` (`self.StaticMesh`) "ECC_Visibility" "ECR_Ignore")))))

(fn `ResetMaterials`
  (for (_array_element _array_index) (`self.OriginalMaterials`)
    (`PrimitiveComponent.SetMaterial` (`self.StaticMesh`) _array_index _array_element)))

(fn `SetMaterialToDynamicInstance`
  (for (_array_element _array_index) (`self.DynamicMaterialsInstances`)
    (`PrimitiveComponent.SetMaterial` (`self.StaticMesh`) _array_index _array_element)))

(fn `UserConstructionScript`
  (`KismetArrayLibrary.Array_Clear` (`self.DynamicMaterialsInstances`))
  (set `self.OriginalMaterials` (`MeshComponent.GetMaterials` (`self.StaticMesh`)))
  (for _array_element (`self.FadeMaterialsInstances`)
    (bind _returnvalue (`KismetMaterialLibrary.CreateDynamicMaterialInstance` _array_element))
    (`KismetArrayLibrary.Array_Add` (`self.DynamicMaterialsInstances`) _returnvalue)))