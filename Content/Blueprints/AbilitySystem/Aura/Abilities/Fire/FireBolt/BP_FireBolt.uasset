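; Fire Bolt projectile actor for the Aura fire ability, with a safeguard against hovering in place when its target dies mid-flight.
; Each Tick compares the projectile movement speed to half of its max speed.
; Below that threshold it spawns the fire explosion Niagara effect and impact sound at its location, then destroys itself.
; BeginPlay, overlap and construction logic are empty in this Blueprint.
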(event `self.ReceiveTick`
  (params (DeltaSeconds :type "Float (single-precision)"))
  (bind _projectilemovement (`self.ProjectileMovement`))
  ;[1 1 1] 当速度低于阈值时销毁,否则会悬停(如飞行物在空中时目标死亡,会停留在目标处
  (if (< (`KismetMathLibrary.VSize` (`MovementComponent.Velocity` _projectilemovement)) (* (`MovementComponent.GetMaxSpeed` _projectilemovement) 0.5))
    (`NiagaraFunctionLibrary.SpawnSystemAtLocation` "/Game/Assets/Effects/Projectiles/FireExplosion/NS_FireExplosion1.NS_FireExplosion1" (`self.K2_GetActorLocation`))
    (`GameplayStatics.SpawnSoundAtLocation` "/Game/Assets/Sounds/Abilities/FireBolt/sfx_FireBolt_Impact.sfx_FireBolt_Impact" (`self.K2_GetActorLocation`) (struct) 1.0 1.0 0.0 null null)
    (`self.K2_DestroyActor`)))

(fn `UserConstructionScript`)