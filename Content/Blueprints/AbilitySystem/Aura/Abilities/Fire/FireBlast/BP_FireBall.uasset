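; Fireball actor for the Fire Blast ability that flies out and returns to its owner like a boomerang.
; StartOutgoingTimeline runs only on authority, lerping the ball along its forward vector to an apex TravelDistance away.
; A second timeline then lerps it from the apex toward the owner's live location.
; Once within ExplodeDistance of the owner, it calls OnHit and destroys itself.
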(event `self.StartOutgoingTimeline`
  (`/Engine/EditorBlueprintResources/ActorMacros.Switch Has Authority`
    (:`Authority`
      (set `self.InitialLocation` (`self.K2_GetActorLocation`))
      (set `self.ApexLocation` (+ (`self.InitialLocation`) (* (`self.GetActorForwardVector`) (`self.TravelDistance`))))
      (bind (_direction _outgoing) (`Timeline|FireBallOutgoing`)
        (:`Update`
          (`self.K2_SetActorLocation` (`KismetMathLibrary.VLerp` (`self.InitialLocation`) (`self.ApexLocation`) _outgoing)))
        (:`Finished`
          (bind (_direction_2 _returning) (`Timeline|FireBallReturning`)
            (:`Update`
              (`self.K2_SetActorLocation` (`KismetMathLibrary.VLerp` (`self.ApexLocation`) (`self.K2_GetActorLocation` (`self.GetOwner`)) _returning))
              (if (<= (`KismetMathLibrary.VSize` (- (`self.K2_GetActorLocation` (`self.GetOwner`)) (`self.K2_GetActorLocation`))) (`self.ExplodeDistance`))
                (`self.OnHit`)
                (`self.K2_DestroyActor`)))))))))

(fn `UserConstructionScript`)