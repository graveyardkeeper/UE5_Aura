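; Gameplay ability for Arcane Shards, a targeted spell that spawns a series of shard effects on the ground.
; It shows a magic circle until input press, then spawns a BP_PointCollection under the mouse to produce randomly rotated ground points.
; The avatar faces the target and plays the cast montage, whose gameplay event starts a looping timer.
; Each tick fires a GameplayCue at the next point; afterwards the collection is destroyed and the ability ends.
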(event `self.K2_ActivateAbility`
  (`|ExecutionSequence`
    (:`then_0`
      ;[1 1 1] 显示技能范围指示器
      (message `PlayerInterface.ShowMagicCircle` (`self.GetAvatarActorFromActorInfo`) null))
    (:`then_1`
      ;[1 1 1] 按键按下，隐藏技能指示器
      (`AbilityTask_WaitInputPress.WaitInputPress` false
        (:`OnPress`
          (message `PlayerInterface.HideMagicCircle` (`self.GetAvatarActorFromActorInfo`))
          ;[1 1 1] 在鼠标位置生成PointCollection，获取NumPoints个技能生成位置
          (bind (_asynctaskproxy _datahandle) (`TargetDataUnderMouse.CreateTargetDataUnderMouse`)
            (:`ValidData`
              (bind _output_get (set `self.MouseTargetLocation` (`.ImpactPoint` (`GameplayStatics.BreakHitResult` (`AbilitySystemBlueprintLibrary.GetHitResultFromTargetData` _datahandle)))))
              (bind _returnvalue (`|SpawnActorFromClass` "/Game/Blueprints/AbilitySystem/Aura/Abilities/Arcane/ArcaneShards/BP_PointCollection.BP_PointCollection_C" (`KismetMathLibrary.MakeTransform` _output_get) "AlwaysSpawn" "MultiplyWithRoot" null null))
              (bind _output_get_2 (set `self.PointCollection` _returnvalue))
              (bind _returnvalue_2 (`PointCollection.GetGroundPoints` _output_get_2 (`self.NumPoints`) (`KismetMathLibrary.RandomFloatInRange` 0.0 360.0)))
              (set `self.GroundPoints` _returnvalue_2)
              ;[1 1 1] 播放施法动画
              (message `CombatInterface.UpdateFacingTarget` (`self.GetAvatarActorFromActorInfo`) (`self.MouseTargetLocation`))
              (`AbilityTask_PlayMontageAndWait.CreatePlayMontageAndWaitProxy` "None" "/Game/Assets/Characters/Aura/Animations/Abilities/AM_Cast_ArcaneShards.AM_Cast_ArcaneShards" 1.0 "None" false
                (:`then`
                  (`AbilityTask_WaitGameplayEvent.WaitGameplayEvent` (struct :`TagName` "Event.Montage.ArcaneShards") null true
                    (:`EventReceived`
                      ;[0.7893 0.483 1] 定时生成每一个奥术碎片，执行GameplayCue特效
                      (bind _returnvalue_3 (`KismetSystemLibrary.K2_SetTimerDelegate` (delegate `SpawnShard`) (`self.ShardSpawnDeltaTime`) true true))
                      (set `self.ShardSpawnTimerHandle` _returnvalue_3)
                      (`self.SpawnShard`))))))))))))

(event `SpawnShard`
  ;[0.7893 0.483 1] 定时生成每一个奥术碎片，执行GameplayCue特效
  (if (< (`self.ShardSpawnIndex`) (`self.NumPoints`))
    (`self.K2_ExecuteGameplayCueWithParams` (struct :`TagName` "GameplayCue.ArcaneShards") (`AbilitySystemBlueprintLibrary.MakeGameplayCueParameters` 0.0 0.0 (struct) (struct) (struct) (struct) (struct) (`SceneComponent.K2_GetComponentLocation` (`|GetArrayItem` (`self.GroundPoints`) (`self.ShardSpawnIndex`)))))
    (`/Engine/EditorBlueprintResources/StandardMacros.IncrementInt` (`self.ShardSpawnIndex`))
    (else
      (`KismetSystemLibrary.K2_ClearAndInvalidateTimerHandle` (`self.ShardSpawnTimerHandle`))
      (`Actor.K2_DestroyActor` (`self.PointCollection`))
      (`KismetSystemLibrary.Delay` 1.0)
      (`self.K2_EndAbility`))))