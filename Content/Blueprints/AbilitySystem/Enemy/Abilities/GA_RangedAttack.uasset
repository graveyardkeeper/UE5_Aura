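; Enemy ranged attack Gameplay Ability that fires a projectile at the avatar's current combat target.
; On activation it turns the avatar toward the target and caches a random tagged montage, since re-evaluation after async nodes would reroll it.
; It plays the montage and waits for its tag's gameplay event, then spawns the projectile from the tagged socket toward the target's current location.
; The ability then ends without stopping the montage.
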(event `self.K2_ActivateAbility`
  (bind _returnvalue (`self.GetAvatarActorFromActorInfo`))
  (bind _returnvalue_2 (message `EnemyInterface.GetCombatTarget` _returnvalue))
  (set `self.CombatTarget` _returnvalue_2)
  (message `CombatInterface.UpdateFacingTarget` _returnvalue (`Actor.K2_GetActorLocation` _returnvalue_2))
  (bind _returnvalue_3 (message `CombatInterface.GetAttackMontages` (`self.GetAvatarActorFromActorInfo`)))
  (bind _output_get (set `self.TaggedMontage` (`self.GetRandomTaggedMontageFromArray` _returnvalue_3))) ; 这里需要把随机到的结果存起来，否则经历后面的异步函数后，会重新求值
  (bind (_montage _montagetag _sockettag) (break `TaggedMontage` _output_get))
  (`AbilityTask_PlayMontageAndWait.CreatePlayMontageAndWaitProxy` "None" _montage 1.0 "None" false
    (:`then`
      (`AbilityTask_WaitGameplayEvent.WaitGameplayEvent` _montagetag null true
        (:`EventReceived`
          (`self.SpawnProjectile` (`Actor.K2_GetActorLocation` (`self.CombatTarget`)) _sockettag (`self.PitchOverride`))
          (`self.K2_EndAbility`))))))