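; Gameplay ability for an enemy summoner that spawns random minions at shuffled spawn locations.
; Activation plays a ground effect at each location and the shaman summon montage, then waits for an attack montage event.
; That event starts a delayed index loop, used because Delay fails inside ForEach, spawning AI-controlled minions one by one.
; The avatar's minion count rises on each spawn and falls when that minion is destroyed.
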(event `self.K2_ActivateAbility`
  (bind _returnvalue (+ (`|GetArrayItem` (`self.SpawnLocations`) (`self.SpawnIndex`)) (0.0 0.0 55.0)))
  (bind _returnvalue_2 (`self.GetSpawnLocations`))
  (bind _output_get (set `self.SpawnLocations` _returnvalue_2))
  (`KismetArrayLibrary.Array_Shuffle` _output_get)
  (for _array_element _output_get
    (`NiagaraFunctionLibrary.SpawnSystemAtLocation` "/Game/Assets/Effects/Combat/NS_GroundSummon.NS_GroundSummon" _array_element))
  (`AbilityTask_PlayMontageAndWait.CreatePlayMontageAndWaitProxy` "None" "/Game/Assets/Enemies/Shaman/Animations/AM_Shaman_Summon.AM_Shaman_Summon"
    (:`then`
      (`AbilityTask_WaitGameplayEvent.WaitGameplayEvent` (struct :`TagName` "Montage.Attack.1") null
        (:`EventReceived`
          ;[0.06789 0.4209 1] 这里不能直接用ForEach，Delay会失效
          (if (< (`self.SpawnIndex`) (`KismetArrayLibrary.Array_Length` (`self.SpawnLocations`))) :!label _label
            (bind _returnvalue_3 (`|SpawnActorFromClass` (`self.GetRandomMinionClass`) (`KismetMathLibrary.MakeTransform` _returnvalue (`KismetMathLibrary.FindLookAtRotation` _returnvalue (`Actor.GetActorForwardVector` (`self.GetAvatarActorFromActorInfo`)))) "AlwaysSpawn" "MultiplyWithRoot" null null))
            (add `Actor.OnDestroyed` _returnvalue_3 (delegate `OnDestroyed_事件`))
            (`Pawn.SpawnDefaultController` _returnvalue_3)
            (`/Engine/EditorBlueprintResources/StandardMacros.IncrementInt` (`self.SpawnIndex`)
              (:`  `
                (message `CombatInterface.IncreaseMinionCount` (`self.GetAvatarActorFromActorInfo`) 1)
                (`KismetSystemLibrary.Delay` 0.2)
                (goto _label)))))))))

(event `OnDestroyed_事件`
  (params (DestroyedActor :type "Actor Object Reference"))
  ;[0.06789 0.4209 1] 这里不能直接用ForEach，Delay会失效
  (message `CombatInterface.IncreaseMinionCount` (`self.GetAvatarActorFromActorInfo`) -1))