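; Melee attack gameplay ability that turns the avatar toward its combat target and damages live players near the strike point.
; It plays a random montage from the avatar's tagged set, cached so async callbacks don't re-roll it.
; The montage's gameplay event triggers a radius query at the tag's combat socket, damaging each player found except the avatar.
; The ability ends after that hit, when the montage finishes or aborts, or if no montages exist.
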(event `self.K2_ActivateAbility`
  (bind _returnvalue (`self.GetAvatarActorFromActorInfo`))
  (bind _returnvalue_2 (`self.GetAvatarActorFromActorInfo`))
  (bind _returnvalue_3 (message `EnemyInterface.GetCombatTarget` _returnvalue_2))
  (bind _ascombat_interface (cast `CombatInterface` _returnvalue_2))
  (`CombatInterface.UpdateFacingTarget` _ascombat_interface (`Actor.K2_GetActorLocation` _returnvalue_3))
  ;[1 0 0.1018] 角色如果配置了多个攻击Montage, 随机播放一个
  (bind _returnvalue_4 (message `CombatInterface.GetAttackMontages` (`self.GetAvatarActorFromActorInfo`)))
  (if (`KismetArrayLibrary.Array_IsEmpty` _returnvalue_4)
    (`self.K2_EndAbility`)
    (else
      (bind _output_get (set `self.TaggedMontage` (`KismetArrayLibrary.Array_Random` _returnvalue_4))) ; 这里需要把随机到的结果存起来，否则经历后面的异步函数后，会重新求值
      (bind (_montage _montagetag) (break `TaggedMontage` _output_get))
      (`AbilityTask_PlayMontageAndWait.CreatePlayMontageAndWaitProxy` "None" _montage
        (:`then`
          (`AbilityTask_WaitGameplayEvent.WaitGameplayEvent` _montagetag null
            (:`EventReceived`
              (bind _returnvalue_5 (message `CombatInterface.GetCombatSocketLocation` _returnvalue _montagetag))
              (bind _outliveplayers (`AuraAbilitySystemLibrary.GetLivePlayersWithinRadius` self (`|MakeArray` _returnvalue) (`self.AttackRadius`) _returnvalue_5))
              (for _array_element _outliveplayers
                (`self.CauseDamage` _array_element))
              (`self.K2_EndAbility`))))
        (:`OnCompleted`
          (`self.K2_EndAbility` :!label _label))
        (:`OnInterrupted`
          (goto _label))
        (:`OnCancelled`
          (goto _label))))))